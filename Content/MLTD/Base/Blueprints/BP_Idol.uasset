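; Idol character actor that assembles its appearance entirely in the construction script from an idol name.
; It scales the body by height and picks body, head and accessory meshes per idol, with optional outfit, accessory and glasses overrides.
; Material overrides on body, face and accessories are cleared after each mesh swap.
; Duplicate body and face meshes follow via master pose, with per-slot flags choosing outline or blank translucent material.
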(fn `ResetMaterials`
  (params (Mesh :type "MeshComponent Object Reference"))
  (`/Engine/EditorBlueprintResources/StandardMacros.IsValid` Mesh
    (:`Is Valid`
      (for (_ _array_index) (`MeshComponent.GetMaterials` Mesh)
        (`PrimitiveComponent.SetMaterial` Mesh _array_index null)))))

(fn `SetIdolAccessories`
  (bind _accessoriesmesh (`self.AccessoriesMesh`))
  (bind _idolglasses (`self.IdolGlasses`))
  (`|ExecutionSequence`
    (:`then_0`
      (`SkinnedMeshComponent.SetSkinnedAssetAndUpdate` (`self.AccessoriesMesh`) null false) ; Clear the mesh by default. Not all idols\nhave head accessories.
      (`/Engine/EditorBlueprintResources/StandardMacros.IsValid` (`self.IdolAccessories`)
        (:`Is Valid`
          (`SkinnedMeshComponent.SetSkinnedAssetAndUpdate` (`self.AccessoriesMesh`) (`self.IdolAccessories`) false))
        (:`Is Not Valid`
          (switch `/Game/MLTD/Base/Blueprints/E_IdolList` (`self.IdolName`)
            (:`NewEnumerator0`
              (`SkinnedMeshComponent.SetSkinnedAssetAndUpdate` _accessoriesmesh "/Game/MLTD/Idols/Haruka/Head/SK_HarukaAccesories.SK_HarukaAccesories" false))
            (:`NewEnumerator4`
              (`SkinnedMeshComponent.SetSkinnedAssetAndUpdate` _accessoriesmesh "/Game/MLTD/Idols/Yayoi/Head/SK_YayoiAccessories.SK_YayoiAccessories" false))
            (:`NewEnumerator6`
              (`SkinnedMeshComponent.SetSkinnedAssetAndUpdate` _accessoriesmesh "/Game/MLTD/Idols/Iori/Head/SK_IoriAccessories.SK_IoriAccessories" false))
            (:`NewEnumerator7`
              (`SkinnedMeshComponent.SetSkinnedAssetAndUpdate` _accessoriesmesh "/Game/MLTD/Idols/Takane/Head/SK_TakaneAccessories.SK_TakaneAccessories" false))
            (:`NewEnumerator8`
              (`SkinnedMeshComponent.SetSkinnedAssetAndUpdate` _accessoriesmesh "/Game/MLTD/Idols/Ritsuko/Head/SK_RitsukoAccessories.SK_RitsukoAccessories" false))
            (:`NewEnumerator10`
              (`SkinnedMeshComponent.SetSkinnedAssetAndUpdate` _accessoriesmesh "/Game/MLTD/Idols/Ami/Head/SK_AmiAccessories.SK_AmiAccessories" false))
            (:`NewEnumerator11`
              (`SkinnedMeshComponent.SetSkinnedAssetAndUpdate` _accessoriesmesh "/Game/MLTD/Idols/Mami/Head/SK_MamiAccessories.SK_MamiAccessories" false))
            (:`NewEnumerator12`
              (`SkinnedMeshComponent.SetSkinnedAssetAndUpdate` _accessoriesmesh "/Game/MLTD/Idols/Hibiki/Head/SK_HibikiAccessories.SK_HibikiAccessories" false))))))
    (:`then_1`
      (`self.ResetMaterials` (`self.AccessoriesMesh`)))
    (:`then_2`
      (`SkinnedMeshComponent.SetSkinnedAssetAndUpdate` (`self.GlassesMesh`) null false) ; Clear the mesh by default. Not all idols\nwear glasses.
      (`/Engine/EditorBlueprintResources/StandardMacros.IsValid` _idolglasses
        (:`Is Valid`
          (`SkinnedMeshComponent.SetSkinnedAssetAndUpdate` (`self.GlassesMesh`) _idolglasses false))))))

(fn `SetIdolBody`
  (bind _bodymesh (`self.BodyMesh`))
  (bind _bodymesh_2 (`self.BodyMesh`))
  (`|ExecutionSequence`
    (:`then_0`
      (`/Engine/EditorBlueprintResources/StandardMacros.IsValid` (`self.IdolOutfit`) ; Use the mesh defined by the variable\nto override. Otherwise, default to the\ncasual outfit.
        (:`Is Valid`
          (`SkinnedMeshComponent.SetSkinnedAssetAndUpdate` (`self.BodyMesh`) (`self.IdolOutfit`) false))
        (:`Is Not Valid`
          (switch `/Game/MLTD/Base/Blueprints/E_IdolList` (`self.IdolName`)
            (:`NewEnumerator0`
              (`SkinnedMeshComponent.SetSkinnedAssetAndUpdate` _bodymesh "/Game/MLTD/Idols/Haruka/Body/SK_HarukaBody.SK_HarukaBody" false))
            (:`NewEnumerator1`
              (`SkinnedMeshComponent.SetSkinnedAssetAndUpdate` _bodymesh_2 "/Game/MLTD/Idols/Chihaya/Body/SK_ChihayaBody.SK_ChihayaBody" false))
            (:`NewEnumerator2`
              (`SkinnedMeshComponent.SetSkinnedAssetAndUpdate` _bodymesh "/Game/MLTD/Idols/Miki/Body/SK_MikiBody.SK_MikiBody" false))
            (:`NewEnumerator3`
              (`SkinnedMeshComponent.SetSkinnedAssetAndUpdate` _bodymesh_2 "/Game/MLTD/Idols/Yukiho/Body/SK_YukihoBody.SK_YukihoBody" false))
            (:`NewEnumerator4`
              (`SkinnedMeshComponent.SetSkinnedAssetAndUpdate` _bodymesh "/Game/MLTD/Idols/Yayoi/Body/SK_YayoiBody.SK_YayoiBody" false))
            (:`NewEnumerator5`
              (`SkinnedMeshComponent.SetSkinnedAssetAndUpdate` _bodymesh_2 "/Game/MLTD/Idols/Makoto/Body/SK_MakotoBody.SK_MakotoBody" false))
            (:`NewEnumerator6`
              (`SkinnedMeshComponent.SetSkinnedAssetAndUpdate` _bodymesh "/Game/MLTD/Idols/Iori/Body/SK_IoriBody.SK_IoriBody" false))
            (:`NewEnumerator7`
              (`SkinnedMeshComponent.SetSkinnedAssetAndUpdate` _bodymesh_2 "/Game/MLTD/Idols/Takane/Body/SK_TakaneBody.SK_TakaneBody" false))
            (:`NewEnumerator8`
              (`SkinnedMeshComponent.SetSkinnedAssetAndUpdate` _bodymesh "/Game/MLTD/Idols/Ritsuko/Body/SK_RitsukoBody.SK_RitsukoBody" false))
            (:`NewEnumerator9`
              (`SkinnedMeshComponent.SetSkinnedAssetAndUpdate` _bodymesh_2 "/Game/MLTD/Idols/Azusa/Body/SK_AzusaBody.SK_AzusaBody" false))
            (:`NewEnumerator10`
              (`SkinnedMeshComponent.SetSkinnedAssetAndUpdate` _bodymesh "/Game/MLTD/Idols/Ami/Body/SK_AmiBody.SK_AmiBody" false))
            (:`NewEnumerator11`
              (`SkinnedMeshComponent.SetSkinnedAssetAndUpdate` _bodymesh_2 "/Game/MLTD/Idols/Mami/Body/SK_MamiBody.SK_MamiBody" false))
            (:`NewEnumerator12`
              (`SkinnedMeshComponent.SetSkinnedAssetAndUpdate` _bodymesh "/Game/MLTD/Idols/Hibiki/Body/SK_HibikiBody.SK_HibikiBody" false))))))
    (:`then_1`
      (`self.ResetMaterials` (`self.BodyMesh`)))))

(fn `SetIdolHead`
  (bind _facemesh (`self.FaceMesh`))
  (bind _facemesh_2 (`self.FaceMesh`))
  (`|ExecutionSequence`
    (:`then_0`
      (switch `/Game/MLTD/Base/Blueprints/E_IdolList` (`self.IdolName`)
        (:`NewEnumerator0`
          (`SkinnedMeshComponent.SetSkinnedAssetAndUpdate` _facemesh_2 "/Game/MLTD/Idols/Haruka/Head/SK_HarukaHead.SK_HarukaHead" false))
        (:`NewEnumerator1`
          (`SkinnedMeshComponent.SetSkinnedAssetAndUpdate` _facemesh "/Game/MLTD/Idols/Chihaya/Head/SK_ChihayaHead.SK_ChihayaHead" false))
        (:`NewEnumerator2`
          (`SkinnedMeshComponent.SetSkinnedAssetAndUpdate` _facemesh_2 "/Game/MLTD/Idols/Miki/Head/SK_MikiHead.SK_MikiHead" false))
        (:`NewEnumerator3`
          (`SkinnedMeshComponent.SetSkinnedAssetAndUpdate` _facemesh "/Game/MLTD/Idols/Yukiho/Head/SK_YukihoHead.SK_YukihoHead" false))
        (:`NewEnumerator4`
          (`SkinnedMeshComponent.SetSkinnedAssetAndUpdate` _facemesh_2 "/Game/MLTD/Idols/Yayoi/Head/SK_YayoiHead.SK_YayoiHead" false))
        (:`NewEnumerator5`
          (`SkinnedMeshComponent.SetSkinnedAssetAndUpdate` _facemesh "/Game/MLTD/Idols/Makoto/Head/SK_MakotoHead.SK_MakotoHead" false))
        (:`NewEnumerator6`
          (`SkinnedMeshComponent.SetSkinnedAssetAndUpdate` _facemesh_2 "/Game/MLTD/Idols/Iori/Head/SK_IoriHead.SK_IoriHead" false))
        (:`NewEnumerator7`
          (`SkinnedMeshComponent.SetSkinnedAssetAndUpdate` _facemesh "/Game/MLTD/Idols/Takane/Head/SK_TakaneHead.SK_TakaneHead" false))
        (:`NewEnumerator8`
          (`SkinnedMeshComponent.SetSkinnedAssetAndUpdate` _facemesh_2 "/Game/MLTD/Idols/Ritsuko/Head/SK_RitsukoHead.SK_RitsukoHead" false))
        (:`NewEnumerator9`
          (`SkinnedMeshComponent.SetSkinnedAssetAndUpdate` _facemesh "/Game/MLTD/Idols/Azusa/Head/SK_AzusaHead.SK_AzusaHead" false))
        (:`NewEnumerator10`
          (`SkinnedMeshComponent.SetSkinnedAssetAndUpdate` _facemesh_2 "/Game/MLTD/Idols/Ami/Head/SK_AmiHead.SK_AmiHead" false))
        (:`NewEnumerator11`
          (`SkinnedMeshComponent.SetSkinnedAssetAndUpdate` _facemesh "/Game/MLTD/Idols/Mami/Head/SK_MamiHead.SK_MamiHead" false))
        (:`NewEnumerator12`
          (`SkinnedMeshComponent.SetSkinnedAssetAndUpdate` _facemesh_2 "/Game/MLTD/Idols/Hibiki/Head/SK_HibikiHead.SK_HibikiHead" false))))
    (:`then_1`
      (`self.ResetMaterials` (`self.FaceMesh`)))))

(fn `SetIdolHeight`
  (`SceneComponent.SetRelativeScale3D` (`self.BodyMesh`) (`KismetMathLibrary.Conv_DoubleToVector` (/ (`KismetMathLibrary.Conv_IntToDouble` (`self.IdolHeight`)) 160.0))))

(fn `SetOutlineMeshes`
  (bind _outline_bodymesh (`self.Outline_BodyMesh`))
  (bind _bodymesh (`self.BodyMesh`))
  (bind _facemesh (`self.FaceMesh`))
  (bind _outline_facemesh (`self.Outline_FaceMesh`))
  (`|ExecutionSequence`
    (:`then_0`
      (`|ExecutionSequence`
        (:`then_0`
          (`SkinnedMeshComponent.SetSkinnedAssetAndUpdate` _outline_bodymesh (`SkinnedMeshComponent.SkeletalMesh` _bodymesh) true)
          (`SkinnedMeshComponent.SetLeaderPoseComponent` _outline_bodymesh _bodymesh true))
        (:`then_1`
          (`SkinnedMeshComponent.SetSkinnedAssetAndUpdate` _outline_facemesh (`SkinnedMeshComponent.SkeletalMesh` _facemesh) true)
          (`SkinnedMeshComponent.SetLeaderPoseComponent` _outline_facemesh _facemesh true))))
    (:`then_1`
      (`|ExecutionSequence`
        (:`then_0`
          (for (_array_element _array_index) (`self.OutfitOutline`)
            (`PrimitiveComponent.SetMaterial` (`self.Outline_BodyMesh`) _array_index (select `bool` _array_element :`false` "/Game/MLTD/Base/Materials/M_BlankTranslucent.M_BlankTranslucent" :`true` "/Game/MLTD/Base/Materials/M_BaseOutline_Inst.M_BaseOutline_Inst" :!type "MaterialInterface Object Reference"))))
        (:`then_1`
          (for (_array_element_2 _array_index_2) (`self.FaceOutline`)
            (`PrimitiveComponent.SetMaterial` (`self.Outline_FaceMesh`) _array_index_2 (select `bool` _array_element_2 :`false` "/Game/MLTD/Base/Materials/M_BlankTranslucent.M_BlankTranslucent" :`true` "/Game/MLTD/Base/Materials/M_BaseOutline_Inst.M_BaseOutline_Inst" :!type "MaterialInterface Object Reference"))))))))

(fn `UserConstructionScript`
  (`self.SetIdolHeight`)
  (`self.SetIdolBody`)
  (`self.SetIdolHead`)
  (`self.SetIdolAccessories`)
  (`self.SetOutlineMeshes`))